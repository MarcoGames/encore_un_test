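; BP_Seasons drives a looping season cycle that controls the Snow scalar in the Season_Parameter material parameter collection.
; Tick uses a one-second Delay as a throttle, slowly advancing Season through a wrapping four-season range before calling SetSeason.
; SetSeason ramps Snow up and back down linearly across the last season, using square root of a square as absolute value, and zeroes it otherwise.
; The construction script also calls SetSeason.
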(event EventBeginPlay)

(event Collision|EventActorBeginOverlap
  (params (OtherActor :type Actor%20Object%20Reference)))

(event EventTick
  (params (DeltaSeconds :type Float%20%28single-precision%29))
  (Utilities|FlowControl|Delay 1.0)
  (Variables|Default|SetSeason (Math|Float|%(Float) (+ (Variables|Default|GetSeason) 0.002) 4.0))
  (CallFunction|SetSeason))

(fn ConstructionScript
  (CallFunction|SetSeason))

(fn SetSeason
  (bind _season (Variables|Default|GetSeason))
  (if (> _season 3.0)
    (Rendering|Material|SetScalarParameterValue "/Game/Environment/Seasons/Season_Parameter.Season_Parameter" "Snow" (- 1.0 (Math|Float|Sqrt (Math|Float|Square (* (- _season 3.5) 2.0)))) :!class /Script/Engine.KismetMaterialLibrary)
    (else
      (Rendering|Material|SetScalarParameterValue "/Game/Environment/Seasons/Season_Parameter.Season_Parameter" "Snow" 0.0 :!class /Script/Engine.KismetMaterialLibrary))))