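; Day-night cycle actor that advances the hour over a configurable day length and updates the lighting.
; Delays on Tick throttle time updates and periodic SkyLight recaptures; the construction script also applies both.
; Cycle converts the hour to sun pitch, whose height samples color curves for the Sky_color parameter collection and fog emissive.
; Height also toggles Sun and Moon and scales sun intensity, while moon intensity is multiplied to zero.
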(event EventBeginPlay
  (Utilities|FlowControl|Sequence
    (:then_0
      (CallFunction|Cycle))
    (:then_1
      (Utilities|FlowControl|Delay 0.1)
      (CallFunction|RecaptureSky))))

(event Collision|EventActorBeginOverlap
  (params (OtherActor :type Actor%20Object%20Reference)))

(event EventTick
  (params (DeltaSeconds :type Float%20%28single-precision%29))
  (bind _update_frequency (Variables|Default|Getupdate%20frequency))
  (Utilities|FlowControl|Sequence
    (:then_0
      (Utilities|FlowControl|Delay _update_frequency)
      (Variables|Default|Setheure (+ (Variables|Default|Getheure) (/ (* _update_frequency 24.0) (Variables|Default|Getday%20duration))))
      (CallFunction|Cycle))
    (:then_1
      (Utilities|FlowControl|Delay 0.7)
      (CallFunction|RecaptureSky))))

(fn ConstructionScript
  (CallFunction|Cycle)
  (CallFunction|RecaptureSky))

(fn Cycle
  ;[1 1 1] convertis l'heure en rotation du soleil
  (Variables|Default|Setsun_rotation (Math|Float|%(Float) (+ (/ (* (Variables|Default|Getheure) 3.6e+02) 24.0) 9e+01) 3.6e+02))
  (Transformation|SetWorldRotation (Variables|Default|GetSun) (Math|Rotator|MakeRotator 0.0 (Variables|Default|Getsun_rotation) 0.0) false false)
  (Variables|Default|Setsun%20height (* (Math|Trig|Sin(Degrees) (Variables|Default|Getsun_rotation)) -1.0))
  ;[0 0.6153 1] Couleur du ciel
  (Rendering|Material|SetVectorParameterValue "/Game/Environment/Sky/Sky_color.Sky_color" "Sky color" (Math|Curves|GetLinearColorValue (Variables|Default|Getsky%20color) (Variables|Default|Getsun%20height)) :!class /Script/Engine.KismetMaterialLibrary)
  (Rendering|Material|SetVectorParameterValue "/Game/Environment/Sky/Sky_color.Sky_color" "Horizon Color" (Math|Curves|GetLinearColorValue (Variables|Default|Gethorizon%20color) (Variables|Default|Getsun%20height)) :!class /Script/Engine.KismetMaterialLibrary)
  (if (>= (Variables|Default|Getsun%20height) 0.0)
    ;[1 1 1] Intensité de la lumière le jour
    (Rendering|Components|Light|SetIntensity (Variables|Default|GetSun) (* (Math|Float|Sqrt (Variables|Default|Getsun%20height)) 5.0))
    (else
      ;[1 1 1] Intensité de la lumière la nuit
      (Rendering|Components|Light|SetIntensity (Variables|Default|GetMoon) (* (Math|Float|Sqrt (* (Variables|Default|Getsun%20height) -1.0)) 0.0))))
  (Rendering|SetVisibility (Variables|Default|GetSun) (not (< (Variables|Default|Getsun%20height) 0.0)) false)
  (Rendering|SetVisibility (Variables|Default|GetMoon) (< (Variables|Default|Getsun%20height) 0.0) false)
  (Class|ExponentialHeightFogComponent|SetVolumetricFogEmissive (Variables|Default|GetExponentialHeightFog) (Math|Curves|GetLinearColorValue (Variables|Default|Getfog%20color) (Variables|Default|Getsun%20height))))

(fn RecaptureSky
  (Class|SkyLightComponent|RecaptureSky (Variables|Default|GetSkyLight)))