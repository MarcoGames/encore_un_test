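; Weather actor that follows the player and drives seasons, cloud cover, rain and fog.
; Chained Delays on Tick stagger updates: clouds step toward a target, Season cycles through four phases, and the target randomly drifts.
; Season yields blend weights, only Winter feeding a material parameter collection; Clouds drives another collection, rain intensity and day-night fog density.
; On BeginPlay it registers with the game instance and BP_eve's Pause.
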(event EventBeginPlay
  (bind _asbp_eve (Utilities|Casting|CastToBP_eve (Game|GetPlayerCharacter 0)))
  (Variables|/Game/HUD/Pause.Pause_C|SetBP_weather%20ref (Variables|/Game/Player/BP_eve.BP_eve_C|GetPause _asbp_eve) self)
  (bind _asbp_game_instance (Utilities|Casting|CastToBP_GameInstance (Game|GetGameInstance)))
  (Variables|/Game/BP_GameInstance.BP_GameInstance_C|SetBP_weather _asbp_game_instance self))

(event Collision|EventActorBeginOverlap
  (params (OtherActor :type Actor%20Object%20Reference)))

(event EventTick
  (params (DeltaSeconds :type Float%20%28single-precision%29))
  (Transformation|SetActorLocation (Transformation|GetActorLocation (Game|GetPlayerCharacter 0)) false false)
  (Utilities|FlowControl|Delay 0.2)
  (CallFunction|SetCloudsIntensity(value))
  (Utilities|FlowControl|Delay 1.0)
  (Variables|Default|SetSeason (Math|Float|%(Float) (+ (Variables|Default|GetSeason) 0.002) 4.0))
  (CallFunction|SetWeather)
  (Utilities|FlowControl|Delay 1e+01)
  (CallFunction|SetCloudsIntensity(target)))

(fn ConstructionScript
  (CallFunction|SetWeather)
  (CallFunction|SetCloudsIntensity))

(fn SetWeather
  (bind _season (Variables|Default|GetSeason))
  (bind _season_2 (Variables|Default|GetSeason))
  (bind _season_3 (Variables|Default|GetSeason))
  (bind _season_4 (Variables|Default|GetSeason))
  (bind _returnvalue (> _season_4 3.0))
  (if (or _returnvalue (< _season_4 1.0))
    (if _returnvalue
      (Variables|Default|Setspring (- (Variables|Default|GetSeason) 3.0))
      (else
        (Variables|Default|Setspring (- 1.0 (Variables|Default|GetSeason)))))
    (else
      (Variables|Default|Setspring 0.0)))
  (if (and (> _season_3 0.0) (< _season_3 2.0))
    (Variables|Default|Setsummer (- 1.0 (Math|Float|Sqrt (Math|Float|Square (- _season_3 1.0)))))
    (else
      (Variables|Default|Setsummer 0.0)))
  (if (and (> _season_2 1.0) (< _season_2 3.0))
    (Variables|Default|Setautumn (- 1.0 (Math|Float|Sqrt (Math|Float|Square (- _season_2 2.0)))))
    (else
      (Variables|Default|Setautumn 0.0)))
  (if (> _season 2.0)
    (Variables|Default|Setwinter (- 1.0 (Math|Float|Sqrt (Math|Float|Square (- _season 3.0)))))
    (else
      (Variables|Default|Setwinter 0.0)))
  (Rendering|Material|SetScalarParameterValue "/Game/Environment/Weather/Weather_parameter.Weather_parameter" "Winter" (Variables|Default|Getwinter) :!class /Script/Engine.KismetMaterialLibrary)
  (Effects|Components|ParticleSystem|SetFloatParameter (Variables|Default|Getrain) "Intensity" (- (Variables|Default|Getclouds) 0.8)))

(fn SetCloudsIntensity(target)
  (bind _output_get (Variables|Default|Settarget%20result (Math|Random|RandomFloatinRange (- (Variables|Default|Getclouds%20intensity%20%28target%29) 0.15) (+ (Variables|Default|Getclouds%20intensity%20%28target%29) 0.15))))
  (if (<= _output_get 0.0)
    (Variables|Default|Setclouds%20intensity%20%28target%29 0.0)
    (elif (>= _output_get 1.0)
      (Variables|Default|Setclouds%20intensity%20%28target%29 1.0)
      (else
        (Variables|Default|Setclouds%20intensity%20%28target%29 _output_get)))))

(fn SetCloudsIntensity(value)
  (if (< (Variables|Default|Getclouds) (Variables|Default|Getclouds%20intensity%20%28target%29))
    (Variables|Default|Setclouds (+ (Variables|Default|Getclouds) 0.005))
    (else
      (Variables|Default|Setclouds (- (Variables|Default|Getclouds) 0.005))))
  (CallFunction|SetCloudsIntensity))

(fn SetCloudsIntensity
  (Rendering|Material|SetScalarParameterValue "/Game/Environment/Sky/Clouds_parameter.Clouds_parameter" "Intensity" (Variables|Default|Getclouds) :!class /Script/Engine.KismetMaterialLibrary)
  (Class|ExponentialHeightFogComponent|SetFogDensity (Variables|/Game/Environment/Sky/BP_day-night.BP_day-night_C|GetExponentialHeightFog (Variables|Default|Getday/night)) (* (Math|Float|Clamp(Float) (- (- 1.0 (Variables|Default|Getclouds)) 0.7) 0.01) 0.2)))