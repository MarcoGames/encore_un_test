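; BP_saveGame is a save-game Blueprint that captures and restores the state of the hero, day/night cycle and weather.
; SaveDefine copies hero stats, movement flags and transform, plus the hour, clouds and season, from the referenced objects into its own variables.
; LoadDefine writes those values back through the same references, repositioning the hero without sweep.
; Neither function writes to or reads from a save slot.
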(fn SaveDefine
  (bind _weather_ref (Variables|Default|GetWeather%20Ref))
  (bind _heroref (Variables|Default|GetHeroRef))
  ;[1 1 1] Save value in BP
  (Variables|Default|SetvieHero (Variables|/Game/Player/BP_eve.BP_eve_C|GetLife _heroref))
  (Variables|Default|SetvieMaxHero (Variables|/Game/Player/BP_eve.BP_eve_C|GetLife_max _heroref))
  (Variables|Default|SetenduranceHero (Variables|/Game/Player/BP_eve.BP_eve_C|Getendurance _heroref))
  (Variables|Default|SetenduranceMaxHero (Variables|/Game/Player/BP_eve.BP_eve_C|GetenduranceMax _heroref))
  (Variables|Default|SetcanRunHero (Variables|/Game/Player/BP_eve.BP_eve_C|GetcanRun _heroref))
  (Variables|Default|SetisCrouchingHero (Variables|/Game/Player/BP_eve.BP_eve_C|GetisCrouching _heroref))
  (Variables|Default|SettransformHero (Transformation|GetActorTransform _heroref))
  (Variables|Default|Setheure (Variables|/Game/Environment/Sky/BP_day-night.BP_day-night_C|Getheure (Variables|Default|GetDay/Night%20cycle%20Ref)))
  (Variables|Default|Setnuages (Variables|/Game/Environment/Weather/BP_Weather.BP_Weather_C|Getclouds _weather_ref))
  (Variables|Default|Setsaison (Variables|/Game/Environment/Weather/BP_Weather.BP_Weather_C|GetSeason _weather_ref)))

(fn LoadDefine
  (bind _weather_ref (Variables|Default|GetWeather%20Ref))
  (bind _heroref (Variables|Default|GetHeroRef))
  (Variables|/Game/Player/BP_eve.BP_eve_C|SetLife _heroref (Variables|Default|GetvieHero))
  (Variables|/Game/Player/BP_eve.BP_eve_C|SetLife_max _heroref (Variables|Default|GetvieMaxHero))
  (Variables|/Game/Player/BP_eve.BP_eve_C|Setendurance _heroref (Variables|Default|GetenduranceHero))
  (Variables|/Game/Player/BP_eve.BP_eve_C|SetenduranceMax _heroref (Variables|Default|GetenduranceMaxHero))
  (Variables|/Game/Player/BP_eve.BP_eve_C|SetcanRun _heroref (Variables|Default|GetcanRunHero))
  (Variables|/Game/Player/BP_eve.BP_eve_C|SetisCrouching _heroref (Variables|Default|GetisCrouchingHero))
  (Transformation|SetActorTransform _heroref (Variables|Default|GettransformHero))
  (Variables|/Game/Environment/Sky/BP_day-night.BP_day-night_C|Setheure (Variables|Default|GetDay/Night%20cycle%20Ref) (Variables|Default|Getheure))
  (Variables|/Game/Environment/Weather/BP_Weather.BP_Weather_C|SetSeason _weather_ref (Variables|Default|Getsaison))
  (Variables|/Game/Environment/Weather/BP_Weather.BP_Weather_C|Setclouds _weather_ref (Variables|Default|Getnuages)))